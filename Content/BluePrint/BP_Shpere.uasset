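; BP_Shpere is a destructible sphere actor that explodes when it takes damage.
; Any damage triggers Die, which spawns an explosion emitter at its location, broadcasts the OnDied dispatcher and destroys the actor.
; The hit, EndPlay and interface print events are empty.
; Disconnected leftover nodes hold explosion and fire effects and a direct BP_GM EndGameCount call, none of which runs.
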(event `self.Sphere.OnComponentHit`
  (params (HitComponent :type "PrimitiveComponent Object Reference") (OtherActor :type "Actor Object Reference") (OtherComp :type "PrimitiveComponent Object Reference") (NormalImpulse :type "Vector Structure") (Hit :type "HitResult Structure (by ref)")))

(event `self.ReceiveEndPlay`
  (params (EndPlayReason :type "EEndPlayReason Enum" :default "Destroyed"))
  ;[1 1 1] 플레이가 끝날시 로케이션에서 이미터(이펙트)를 실행시킨다
)

(event `self.ReceiveAnyDamage`
  (params (Damage :type "Float (single-precision)") (DamageType :type "DamageType Object Reference") (InstigatedBy :type "Controller Object Reference") (DamageCauser :type "Actor Object Reference"))
  ;[1 1 1] 데미지를 받으면 다이를 실행
  (`self.Die`))

(event `/Game/BluePrint/Interfaces/IF_print.Interfaceprint`)

(event `Die`
  ;[1 1 1] 로케이션에 있는 액터가 파괴되면 콜을 준다.
  (`GameplayStatics.SpawnEmitterAtLocation` "/Game/StarterContent/Particles/P_Explosion.P_Explosion" (`self.K2_GetActorLocation`))
  (`self.OnDied`)
  (`self.K2_DestroyActor`))

(fn `UserConstructionScript`)